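; Actor Blueprint that plays background songs in a continuous random shuffle.
; On BeginPlay it picks a random entry from SongList, assigns it to the Audio component and plays it.
; It then waits for that sound's duration and calls PlaySong again, looping indefinitely with possible immediate repeats.
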(event Custom|PlaySong
  (Audio|Components|Audio|SetSound (Variables|Default|GetAudio) (Utilities|Array|Get(acopy) (Variables|Default|GetSongList) (Math|Random|RandomIntegerinRange 0 (- (Utilities|Array|Length (Variables|Default|GetSongList)) 1))))
  (Audio|Components|Audio|Play (Variables|Default|GetAudio) 0.0)
  (Utilities|FlowControl|Delay (Variables|/Script/Engine.SoundBase|GetDuration (Variables|/Script/Engine.AudioComponent|GetSound (Variables|Default|GetAudio))))
  (CallFunction|PlaySong))

(event EventBeginPlay
  (CallFunction|PlaySong))

(fn ConstructionScript)