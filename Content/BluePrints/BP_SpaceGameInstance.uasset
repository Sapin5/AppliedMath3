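; Game instance for a space game that holds the player's score and ship handling settings across levels.
; Score functions add points to the running total or reset it to zero.
; SetDifficulty switches on a Slow, Medium or Fast speed choice to set left/right and up/down turn rates plus acceleration, with faster tiers raising all three.
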(fn UpdatePlayerScore
  (params (PointValue :type Integer))
  (Variables|Default|SetPlayerScore (+ PointValue (Variables|Default|GetPlayerScore))))

(fn ResetPlayerScore
  (Variables|Default|SetPlayerScore 0))

(fn SetDifficulty
  (params (Speed :type Difficulty%20Enum :default "NewEnumerator0"))
  (switch Utilities|FlowControl|Switch|SwitchonDifficulty Speed
    (:NewEnumerator0
      (Variables|Default|SetTurnSpeedLR 0.3)
      (Variables|Default|SetTurnSpeedUD 0.1)
      (Variables|Default|SetAccelSpeed 2e+01))
    (:NewEnumerator1
      (Variables|Default|SetTurnSpeedLR 0.4)
      (Variables|Default|SetTurnSpeedUD 0.2)
      (Variables|Default|SetAccelSpeed 3e+01))
    (:NewEnumerator2
      (Variables|Default|SetTurnSpeedLR 0.6)
      (Variables|Default|SetTurnSpeedUD 0.4)
      (Variables|Default|SetAccelSpeed 4e+01))))