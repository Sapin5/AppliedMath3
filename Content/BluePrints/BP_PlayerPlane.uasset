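; Player-controlled plane pawn with Enhanced Input flight, twin guns and a HUD showing speed and active inputs.
; Thrust builds a velocity vector that Tick reduces by squared-velocity drag and applies as an unswept world offset.
; A shared logistic S-curve shapes thrust, pitch and the delayed camera follow, which right-mouse free look suspends.
; Rate-limited fire spawns projectiles from both guns, adding doubled plane velocity to bullet speed.
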(event OnComponentBeginOverlap(Capsule)
  (params (OverlappedComponent :type Primitive%20Component%20Object%20Reference) (OtherActor :type Actor%20Object%20Reference) (OtherComp :type Primitive%20Component%20Object%20Reference) (OtherBodyIndex :type Integer) (bFromSweep :type Boolean) (SweepResult :type Hit%20Result%20Structure%20%28by%20ref%29)))

(event Input|EnhancedActionEvents|EnhancedInputActionIA_Look
  (params (ActionValue :type Vector%202D%20Structure) (ElapsedSeconds :type Float%20%28double-precision%29) (TriggeredSeconds :type Float%20%28double-precision%29) (InputAction :type Input%20Action%20Object%20Reference :default "/Game/InputSystem/IA_Look.IA_Look"))
  (if (Variables|Camera|GetbLook%20around)
    (Transformation|AddLocalRotation (Variables|Default|GetSpringArm) (Math|Rotator|MakeRotator 0.0 (.y ActionValue) (.x ActionValue)) false false)))

(event Input|EnhancedActionEvents|EnhancedInputActionIA_Down
  (params (ActionValue :type Boolean) (ElapsedSeconds :type Float%20%28double-precision%29) (TriggeredSeconds :type Float%20%28double-precision%29) (InputAction :type Input%20Action%20Object%20Reference :default "/Game/InputSystem/IA_Down.IA_Down"))
  (:Triggered
    (Variables|Default|SetRotate%20Speed%20Vertical (/ (+ ElapsedSeconds (Variables|Default|GetRotate%20Speed%20Vertical)) 1.5))
    (Transformation|AddLocalRotation (Variables|Default|GetPlane) (Math|Rotator|MakeRotator 0.0 (CallFunction|SCurve 1.0 1.0 (Variables|Default|GetRotate%20Speed%20Vertical) 0.0) 0.0) false false)
    (Variables|Camera|SetAlphaCamera 0.5)
    (Widget|SetIsEnabled (Variables|/Game/BluePrints/WB_HUD.WB_HUD_C|GetIA_Down (Variables|Default|GetWidgetRef)) ActionValue :!label _label))
  (:Completed
    (Variables|Default|SetRotate%20Speed%20Vertical 0.0)
    (goto _label)))

(event Input|EnhancedActionEvents|EnhancedInputActionIA_Forwards
  (params (ActionValue :type Boolean) (ElapsedSeconds :type Float%20%28double-precision%29) (TriggeredSeconds :type Float%20%28double-precision%29) (InputAction :type Input%20Action%20Object%20Reference :default "/Game/InputSystem/IA_Forwards.IA_Forwards"))
  (:Triggered
    (Variables|Speed|SetAcceleration (+ (Variables|Speed|GetAcceleration) TriggeredSeconds))
    (Variables|Speed|SetVelocity (CallFunction|SetVelocity (CallFunction|SCurve 2.0 0.008 (+ (Variables|Speed|GetAcceleration) TriggeredSeconds) 2e+02))))
  (:Completed
    (Variables|Speed|SetAcceleration 0.0)))

(event Input|EnhancedActionEvents|EnhancedInputActionIA_Left
  (params (ActionValue :type Boolean) (ElapsedSeconds :type Float%20%28double-precision%29) (TriggeredSeconds :type Float%20%28double-precision%29) (InputAction :type Input%20Action%20Object%20Reference :default "/Game/InputSystem/IA_Left.IA_Left"))
  (:Triggered
    (Transformation|AddLocalRotation (Variables|Default|GetPlane) "0.000000,-0.300000,0.000000" false false)
    (Variables|Camera|SetAlphaCamera 0.5)
    (Widget|SetIsEnabled (Variables|/Game/BluePrints/WB_HUD.WB_HUD_C|GetIA_Left (Variables|Default|GetWidgetRef)) ActionValue :!label _label))
  (:Completed
    (goto _label)))

(event Input|EnhancedActionEvents|EnhancedInputActionIA_Right
  (params (ActionValue :type Boolean) (ElapsedSeconds :type Float%20%28double-precision%29) (TriggeredSeconds :type Float%20%28double-precision%29) (InputAction :type Input%20Action%20Object%20Reference :default "/Game/InputSystem/IA_Right.IA_Right"))
  (:Triggered
    (Transformation|AddLocalRotation (Variables|Default|GetPlane) "0.000000,0.300000,0.000000" false false)
    (Variables|Camera|SetAlphaCamera 0.5)
    (Widget|SetIsEnabled (Variables|/Game/BluePrints/WB_HUD.WB_HUD_C|GetIA_Right (Variables|Default|GetWidgetRef)) ActionValue :!label _label))
  (:Completed
    (goto _label)))

(event Input|EnhancedActionEvents|EnhancedInputActionIA_Up
  (params (ActionValue :type Boolean) (ElapsedSeconds :type Float%20%28double-precision%29) (TriggeredSeconds :type Float%20%28double-precision%29) (InputAction :type Input%20Action%20Object%20Reference :default "/Game/InputSystem/IA_Up.IA_Up"))
  (:Triggered
    (Variables|Default|SetRotate%20Speed%20Vertical (/ (+ ElapsedSeconds (Variables|Default|GetRotate%20Speed%20Vertical)) 1.5))
    (Transformation|AddLocalRotation (Variables|Default|GetPlane) (Math|Rotator|MakeRotator 0.0 (CallFunction|SCurve -1.0 1.0 (Variables|Default|GetRotate%20Speed%20Vertical) 0.0) 0.0) false false)
    (Variables|Camera|SetAlphaCamera 0.5)
    (Widget|SetIsEnabled (Variables|/Game/BluePrints/WB_HUD.WB_HUD_C|GetIA_UP (Variables|Default|GetWidgetRef)) ActionValue :!label _label))
  (:Completed
    (Variables|Default|SetRotate%20Speed%20Vertical 0.0)
    (goto _label)))

(event Input|EnhancedActionEvents|EnhancedInputActionIA_RollLeft
  (params (ActionValue :type Boolean) (ElapsedSeconds :type Float%20%28double-precision%29) (TriggeredSeconds :type Float%20%28double-precision%29) (InputAction :type Input%20Action%20Object%20Reference :default "/Game/InputSystem/IA_RollLeft.IA_RollLeft"))
  (Transformation|AddLocalRotation (Variables|Default|GetPlane) "0.0,0.0,-1.000000" false false)
  (Variables|Camera|SetAlphaCamera 0.5)
  (Widget|SetIsEnabled (Variables|/Game/BluePrints/WB_HUD.WB_HUD_C|GetIA_RollLeft (Variables|Default|GetWidgetRef)) ActionValue))

(event Input|EnhancedActionEvents|EnhancedInputActionIA_Fire
  (params (ActionValue :type Boolean) (ElapsedSeconds :type Float%20%28double-precision%29) (TriggeredSeconds :type Float%20%28double-precision%29) (InputAction :type Input%20Action%20Object%20Reference :default "/Game/InputSystem/IA_Fire.IA_Fire"))
  (:Triggered
    (bind _output_get (Variables|Gun|SetTimeSinceLastShot (+ (Variables|Default|GetDelta%20Seconds) (Variables|Gun|GetTimeSinceLastShot))))
    (if (> _output_get (Variables|Gun|GetFireRate))
      (Variables|Gun|SetTimeSinceLastShot 0.0)
      (bind _returnvalue (Game|SpawnActorfromClass "/Game/BluePrints/BP_Projectile.BP_Projectile_C" (Transformation|GetWorldTransform (Variables|Default|GetGunRight)) "AlwaysSpawn" "MultiplyWithRoot" 0 0))
      (Default|SetBulletVelocity _returnvalue (CallFunction|GetBulletVelocity (Variables|Default|GetGunRight)))
      (bind _returnvalue_2 (Game|SpawnActorfromClass "/Game/BluePrints/BP_Projectile.BP_Projectile_C" (Transformation|GetWorldTransform (Variables|Default|GetGunLeft)) "AlwaysSpawn" "MultiplyWithRoot" 0 0))
      (Default|SetBulletVelocity _returnvalue_2 (CallFunction|GetBulletVelocity (Variables|Default|GetGunLeft)))))
  (:Completed
    (Variables|Gun|SetTimeSinceLastShot 0.4)))

(event Input|EnhancedActionEvents|EnhancedInputActionIA_RollRight
  (params (ActionValue :type Boolean) (ElapsedSeconds :type Float%20%28double-precision%29) (TriggeredSeconds :type Float%20%28double-precision%29) (InputAction :type Input%20Action%20Object%20Reference :default "/Game/InputSystem/IA_RollRight.IA_RollRight"))
  (Transformation|AddLocalRotation (Variables|Default|GetPlane) "0.0,0.0,1.000000" false false)
  (Variables|Camera|SetAlphaCamera 0.5)
  (Widget|SetIsEnabled (Variables|/Game/BluePrints/WB_HUD.WB_HUD_C|GetIA_RollRight (Variables|Default|GetWidgetRef)) ActionValue))

(event EventBeginPlay
  (Utilities|FlowControl|Sequence
    (:then_0
      (bind _asplayer_controller (Utilities|Casting|CastToPlayerController (Pawn|GetController)))
      (Input|AddMappingContext (PlayerController|LocalPlayerSubsystems|GetEnhancedInputLocalPlayerSubsystem _asplayer_controller) "/Game/InputSystem/IMC_ShipControls.IMC_ShipControls" 0 "(bIgnoreAllPressedKeysUntilRelease=True,bForceImmediately=False,bNotifyUserSettings=False)"))
    (:then_1
      (Physics|SetEnableGravity (Variables|Default|GetPlane) false))
    (:then_2
      (Variables|Default|SetField%20Of%20View (Variables|/Script/Engine.CameraComponent|GetFieldOfView (Variables|Default|GetPlayerView))))
    (:then_3
      (bind _returnvalue (UserInterface|CreateWidget "/Game/BluePrints/WB_HUD.WB_HUD_C" (Game|GetPlayerController 0)))
      (bind _output_get (Variables|Default|SetWidgetRef _returnvalue))
      (UserInterface|Viewport|AddtoViewport _output_get 0))))

(event EventTick
  (params (DeltaSeconds :type Float%20%28single-precision%29))
  (bind _output_get (Variables|Default|SetDelta%20Seconds DeltaSeconds))
  (Utilities|FlowControl|Sequence
    (:then_0
      (CallFunction|MovePlayer)
      (if (Variables|Default|GetbDebug)
        _
        (else
          (Development|PrintText (|CollapseGraph_1) true false "(R=0.000000,G=0.660000,B=1.000000,A=1.000000)" 1e+01 "Player Velocity")
          (Development|PrintText (|CollapseGraph_0) true true "(R=0.000000,G=0.660000,B=1.000000,A=1.000000)" 2.0 "Magnitude")
          (Development|PrintText (|CollapseGraph) true true "(R=0.000000,G=0.660000,B=1.000000,A=1.000000)" 2.0 "Rotation")))
      (Default|SetInputText (Variables|Default|GetWidgetRef) (CallFunction|NewFunction)))
    (:then_1
      (if (Variables|Camera|GetbLook%20around)
        (Variables|Camera|SetAlphaCamera 0.0)
        (else
          (CallFunction|CameraDelay _output_get))))
    (:then_2
      (Camera|SetFieldOfView (Variables|Default|GetPlayerView) 1.1e+02))))

(event Input|MouseEvents|RightMouseButton
  (params (Key :type Key%20Structure :default "None"))
  (:Pressed
    (Variables|Camera|SetbLook%20around true))
  (:Released
    (Variables|Camera|SetbLook%20around false)))

(fn ConstructionScript)

(fn SetVelocity
  (params (B :type Float%20%28double-precision%29))
  (return (+ (* (Math|Vector|GetForwardVector (Variables|Default|GetPlane)) B) (Variables|Speed|GetVelocity))))

(fn Drag
  (return (+ (* (Math|Vector|VectorLength (* (Variables|Speed|GetDragTime) (* (Variables|Speed|Getc) (* (Variables|Speed|GetVelocity) (Variables|Speed|GetVelocity))))) (Math|Vector|Normalize (* (Variables|Speed|GetVelocity) -1.0))) (Variables|Speed|GetVelocity))))

(fn SCurve
  (params (Curve%20Height%20%28J%29 :type Float%20%28double-precision%29) (Curve%20Slope%20%28I%29 :type Float%20%28double-precision%29) (X%20Value :type Float%20%28double-precision%29) (Starting%20Point%20%28S%29 :type Float%20%28double-precision%29))
  (return (/ Curve%20Height%20%28J%29 (+ (Math|Float|Power 2.71828 (* (* Curve%20Slope%20%28I%29 -1.0) (- X%20Value Starting%20Point%20%28S%29))) 1.0))))

(fn CameraDelay
  (params (B :type Float%20%28double-precision%29))
  (bind _referencecone (Variables|Default|GetReferenceCone))
  (bind _returnvalue (Transformation|GetWorldRotation _referencecone))
  (Variables|Camera|SetAlphaCamera (+ (Variables|Camera|GetAlphaCamera) B))
  (Transformation|SetWorldRotation (Variables|Default|GetSpringArm) (Math|Rotator|Lerp(Rotator) (Transformation|GetWorldRotation (Variables|Default|GetSpringArm)) (Math|Rotator|MakeRotator (.roll _returnvalue) (.pitch _returnvalue) (.yaw _returnvalue)) (CallFunction|SCurve 1.0 2.0 (Variables|Camera|GetAlphaCamera) 2.0) true) false false))

(fn NewFunction
  (bind _output_get (Variables|Speed|SetVelocityMag (Math|Conversions|ToFloat(Integer) (Math|Float|Round (* (Math|Vector|VectorLength (Variables|Speed|GetVelocity)) 1e+01)))))
  (return (Utilities|Text|ToText(Float) _output_get "HalfToEven")))

(fn MovePlayer
  (Variables|Speed|SetDragTime (Variables|Default|GetDelta%20Seconds))
  (bind _output_get (Variables|Speed|SetVelocity (CallFunction|Drag)))
  (Transformation|AddActorWorldOffset self _output_get))

(fn GetBulletVelocity
  (params (GunReference :type Scene%20Component%20Object%20Reference))
  (return (+ (* (Variables|Speed|GetVelocity) 2.0) (* (Math|Vector|GetForwardVector GunReference) (Variables|Gun|GetBulletSpeed)))))