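; Comet manager that keeps a set of small, medium and large comets active in random spots around the world origin, using object pools.
; BeginPlay pre-spawns hidden comets per size, then activates random ones.
; Tick manually updates only comets within mesh cull distance of the player plane, swapping collided ones for random pooled replacements.
; An out-of-bounds relocation check exists but compares two zero vectors, so it never fires.
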(event EventBeginPlay
  (Utilities|FlowControl|Sequence
    (:then_0
      (Variables|Default|SetPoolTransform (Transformation|GetWorldTransform (Variables|Default|GetDefaultSceneRoot)))
      (bind _asbp_player_plane (Utilities|Casting|CastToBP_PlayerPlane (Game|Player|GetPlayerPawn 0)))
      (Variables|Default|SetBP%20Player%20Plane _asbp_player_plane))
    (:then_1
      (for _index (range 0 (- (Variables|Default|GetMaxPoolSize) 1))
        (bind _returnvalue (Game|SpawnActorfromClass "/Game/BluePrints/Comets/BP_Comet_Small.BP_Comet_Small_C" (Variables|Default|GetPoolTransform) "Undefined" "MultiplyWithRoot" 0 false 0))
        (CallFunction|HideActor _returnvalue (Variables|/Game/BluePrints/Comets/BP_Comet_Small.BP_Comet_Small_C|GetSphere _returnvalue))
        (Utilities|Array|Add (Variables|Default|GetSmallCometPool) _returnvalue)
        (bind _returnvalue_2 (Game|SpawnActorfromClass "/Game/BluePrints/Comets/BP_Comet_Medium.BP_Comet_Medium_C" (Variables|Default|GetPoolTransform) "Undefined" "MultiplyWithRoot" 0 false 0))
        (CallFunction|HideActor _returnvalue_2 (Variables|/Game/BluePrints/Comets/BP_Comet_Medium.BP_Comet_Medium_C|GetSphere _returnvalue_2))
        (Utilities|Array|Add (Variables|Default|GetMediumCometPool) _returnvalue_2)
        (bind _returnvalue_3 (Game|SpawnActorfromClass "/Game/BluePrints/Comets/BP_Comet_Large.BP_Comet_Large_C" (Variables|Default|GetPoolTransform) "Undefined" "MultiplyWithRoot" 0 false 0))
        (CallFunction|HideActor _returnvalue_3 (Variables|/Game/BluePrints/Comets/BP_Comet_Large.BP_Comet_Large_C|GetBox _returnvalue_3))
        (Utilities|Array|Add (Variables|Default|GetLargeCometPool) _returnvalue_3)))
    (:then_2
      (for _index_2 (range 0 (- (Variables|Default|GetMaxActivePoolSize) 1))
        (bind _pooledactor (CallFunction|GetPooledActor (.OutItem (Utilities|Array|Random (Variables|Default|GetCometEnum))) (CallFunction|GetRandomSpawnPoint)))
        (Utilities|Array|Add (Variables|Default|GetPooledActors) _pooledactor)))))

(event EventTick
  (params (DeltaSeconds :type Float%20%28single-precision%29))
  (Variables|Default|SetDelta%20Seconds DeltaSeconds)
  (CallFunction|TickComets))

(fn ConstructionScript)

(fn GetPooledActor
  (params (NewParam :type CometType%20Enum :default "NewEnumerator0") (Transform :type Transform))
  (bind (_location _rotation) (Math|Transform|BreakTransform Transform))
  (bind _smallcometpool (Variables|Default|GetSmallCometPool))
  (bind _largecometpool (Variables|Default|GetLargeCometPool))
  (bind _mediumcometpool (Variables|Default|GetMediumCometPool))
  (switch Utilities|FlowControl|Switch|SwitchonCometType NewParam
    (:NewEnumerator0
      (if (> (Utilities|Array|Length _smallcometpool) 0)
        (bind _output_get (Variables|Default|SetPooledObject (Utilities|Array|Get(acopy) _smallcometpool)))
        (bind _asbp_comet_small (Utilities|Casting|CastToBP_Comet_Small _output_get))
        (Utilities|Array|RemoveItem (Variables|Default|GetSmallCometPool) _asbp_comet_small)
        (Variables|/Game/BluePrints/Comets/BP_Comet_Small.BP_Comet_Small_C|SetbCollided _asbp_comet_small false)
        (Collision|SetCollisionEnabled (Variables|/Game/BluePrints/Comets/BP_Comet_Small.BP_Comet_Small_C|GetSphere _asbp_comet_small) "QueryOnly")
        (Transformation|Teleport (Variables|Default|GetPooledObject) _location _rotation :!label _label)
        (Rendering|SetActorHiddenInGame (Variables|Default|GetPooledObject) false)
        (return (Variables|Default|GetPooledObject))))
    (:NewEnumerator1
      (if (> (Utilities|Array|Length _mediumcometpool) 0)
        (bind _output_get_2 (Variables|Default|SetPooledObject (Utilities|Array|Get(acopy) _mediumcometpool)))
        (bind _asbp_comet_medium (Utilities|Casting|CastToBP_Comet_Medium _output_get_2))
        (Utilities|Array|RemoveItem (Variables|Default|GetMediumCometPool) _asbp_comet_medium)
        (Variables|/Game/BluePrints/Comets/BP_Comet_Medium.BP_Comet_Medium_C|SetbCollided _asbp_comet_medium false)
        (Collision|SetCollisionEnabled (Variables|/Game/BluePrints/Comets/BP_Comet_Medium.BP_Comet_Medium_C|GetSphere _asbp_comet_medium) "QueryOnly")
        (goto _label)))
    (:NewEnumerator2
      (if (> (Utilities|Array|Length _largecometpool) 0)
        (bind _output_get_3 (Variables|Default|SetPooledObject (Utilities|Array|Get(acopy) _largecometpool)))
        (bind _asbp_comet_large (Utilities|Casting|CastToBP_Comet_Large _output_get_3))
        (Utilities|Array|RemoveItem (Variables|Default|GetLargeCometPool) _asbp_comet_large)
        (Variables|/Game/BluePrints/Comets/BP_Comet_Large.BP_Comet_Large_C|SetbCollided _asbp_comet_large false)
        (Collision|SetCollisionEnabled (Variables|/Game/BluePrints/Comets/BP_Comet_Large.BP_Comet_Large_C|GetBox _asbp_comet_large) "QueryOnly")
        (goto _label)))))

(fn TickComets
  (for _array_element (Variables|Default|GetPooledActors)
    (bind _output_get (LocalVariables|SetCurrentActor _array_element))
    (CallFunction|CheckCometsLocation _output_get)
    (bind _asbp_comet_small (Utilities|Casting|CastToBP_Comet_Small (LocalVariables|GetCurrentActor))
      (:then
        (bind _output_get_2 (LocalVariables|SetSmallComet _asbp_comet_small))
        (if (not (CallFunction|DistanceBetweenCometandPlayer (Variables|/Game/BluePrints/Comets/BP_Comet_Small.BP_Comet_Small_C|GetComit _output_get_2)))
          (Default|TickComet (LocalVariables|GetSmallComet) (Variables|Default|GetDelta%20Seconds))
          (if (Variables|/Game/BluePrints/Comets/BP_Comet_Small.BP_Comet_Small_C|GetbCollided (LocalVariables|GetSmallComet))
            (Utilities|Array|RemoveItem (Variables|Default|GetPooledActors) (LocalVariables|GetCurrentActor))
            (Utilities|Array|Add (Variables|Default|GetSmallCometPool) (LocalVariables|GetSmallComet))
            (Rendering|SetActorHiddenInGame (LocalVariables|GetCurrentActor) true)
            (Development|PrintText (Utilities|Text|FormatText "Comet: {c} hit 
Removing from tick group" (LocalVariables|GetCurrentActor)) :!label _label)
            (Transformation|Teleport (LocalVariables|GetCurrentActor) (.Location (Math|Transform|BreakTransform (Variables|Default|GetPoolTransform))) "0, 0, 0")
            (bind _pooledactor (CallFunction|GetPooledActor (.OutItem (Utilities|Array|Random (Variables|Default|GetCometEnum))) (CallFunction|GetRandomSpawnPoint)))
            (if (Variables|Default|GetbDebug)
              (Development|PrintText (Utilities|Text|FormatText "Actor: {A} Has been added to active comet pool" _pooledactor)))
            (Utilities|Array|Add (Variables|Default|GetPooledActors) _pooledactor))))
      (:CastFailed
        (bind _asbp_comet_medium (Utilities|Casting|CastToBP_Comet_Medium (LocalVariables|GetCurrentActor))
          (:then
            (bind _output_get_3 (LocalVariables|SetMedium%20Comet _asbp_comet_medium))
            (if (not (CallFunction|DistanceBetweenCometandPlayer (Variables|/Game/BluePrints/Comets/BP_Comet_Medium.BP_Comet_Medium_C|GetComet _output_get_3)))
              (Default|TickComet (LocalVariables|GetMedium%20Comet) (Variables|Default|GetDelta%20Seconds))
              (if (Variables|/Game/BluePrints/Comets/BP_Comet_Medium.BP_Comet_Medium_C|GetbCollided (LocalVariables|GetMedium%20Comet))
                (Utilities|Array|RemoveItem (Variables|Default|GetPooledActors) (LocalVariables|GetCurrentActor))
                (Utilities|Array|Add (Variables|Default|GetMediumCometPool) (LocalVariables|GetMedium%20Comet))
                (Rendering|SetActorHiddenInGame (LocalVariables|GetCurrentActor) true)
                (goto _label))))
          (:CastFailed
            (bind _asbp_comet_large (Utilities|Casting|CastToBP_Comet_Large (LocalVariables|GetCurrentActor)))
            (bind _output_get_4 (LocalVariables|SetLarge%20Comet _asbp_comet_large))
            (if (not (CallFunction|DistanceBetweenCometandPlayer (Variables|/Game/BluePrints/Comets/BP_Comet_Large.BP_Comet_Large_C|GetComet _output_get_4)))
              (Default|TickComet (LocalVariables|GetLarge%20Comet) (Variables|Default|GetDelta%20Seconds))
              (if (Variables|/Game/BluePrints/Comets/BP_Comet_Large.BP_Comet_Large_C|GetbCollided (LocalVariables|GetLarge%20Comet))
                (Utilities|Array|RemoveItem (Variables|Default|GetPooledActors) (LocalVariables|GetCurrentActor))
                (Utilities|Array|Add (Variables|Default|GetLargeCometPool) (LocalVariables|GetLarge%20Comet))
                (Rendering|SetActorHiddenInGame (LocalVariables|GetCurrentActor) true)
                (goto _label)))))))))

(fn GetRandomSpawnPoint
  (return (Math|Transform|MakeTransform (Math|Vector|MakeVector (Math|Random|RandomFloatinRange -4e+04 4e+04) (Math|Random|RandomFloatinRange -4e+04 4e+04) (Math|Random|RandomFloatinRange -4e+04 4e+04)) (Math|Rotator|MakeRotator (Math|Random|RandomFloatinRange 0.0 3.6e+02) (Math|Random|RandomFloatinRange 0.0 3.6e+02) (Math|Random|RandomFloatinRange 0.0 3.6e+02)))))

(fn HideActor
  (params (ActorRef :type Actor%20Object%20Reference) (ColliderRef :type Primitive%20Component%20Object%20Reference))
  (Rendering|SetActorHiddenInGame ActorRef true)
  (Collision|SetCollisionEnabled ColliderRef "NoCollision"))

(fn CheckCometsLocation
  (params (ActorRef :type Actor%20Object%20Reference))
  (if (> (Math|Vector|Distance(Vector) "0, 0, 0" "0, 0, 0") 4e+04)
    (Variables|Default|SetNewVar (Math|Vector|MakeVector (Math|Random|RandomFloatinRange -4e+04 4e+04) (Math|Random|RandomFloatinRange -4e+04 4e+04) (Math|Random|RandomFloatinRange -4e+04 4e+04)))
    (Rendering|SetActorHiddenInGame ActorRef true)
    (Development|PrintText (|CollapseGraph))
    (Transformation|SetActorLocation ActorRef (Variables|Default|GetNewVar) false true)
    (Rendering|SetActorHiddenInGame ActorRef false)
    (Development|PrintText (Utilities|Text|FormatText "Actor {A} Has Been teleported" ActorRef)))
  (return))

(fn DistanceBetweenCometandPlayer
  (params (CometRef :type Instanced%20Static%20Mesh%20Component%20Object%20Reference))
  (return (< (.OutEndCullDistance (Class|InstancedStaticMeshComponent|GetCullDistances CometRef)) (Math|Vector|Distance(Vector) (Transformation|GetWorldLocation CometRef) (Transformation|GetActorLocation (Variables|Default|GetBP%20Player%20Plane))))))