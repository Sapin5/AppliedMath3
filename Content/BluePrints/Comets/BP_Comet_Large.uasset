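; BP_Comet_Large is a comet actor that drifts in a random direction and registers hits from the player plane or projectiles.
; Construction picks a random mesh, applies a material and adds an instance to the Comet component.
; BeginPlay randomly rotates Comet and derives Velocity from its forward vector and Speed.
; A TickComet event applies that as a delta-time-scaled local offset, while Box overlaps with BP_PlayerPlane or BP_Projectile only set Collided.
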(event OnComponentBeginOverlap(Box)
  (params (OverlappedComponent :type Primitive%20Component%20Object%20Reference) (OtherActor :type Actor%20Object%20Reference) (OtherComp :type Primitive%20Component%20Object%20Reference) (OtherBodyIndex :type Integer) (bFromSweep :type Boolean) (SweepResult :type Hit%20Result%20Structure%20%28by%20ref%29))
  (Utilities|FlowControl|Sequence
    (:then_0
      (Utilities|Casting|CastToBP_PlayerPlane OtherActor))
    (:then_1
      (Utilities|Casting|CastToBP_Projectile OtherActor)))
  (Variables|Default|SetbCollided true))

(event Custom|TickComet
  (params (DeltaTme :type Float%20%28double-precision%29))
  (Transformation|AddActorLocalOffset (* DeltaTme (Variables|Default|GetVelocity)) false false))

(event EventBeginPlay
  (bind _comet (Variables|Default|GetComet))
  (Transformation|SetWorldRotation _comet (Math|Rotator|MakeRotator (Math|Random|RandomFloatinRange 0.0 365.0) (Math|Random|RandomFloatinRange 0.0 365.0) (Math|Random|RandomFloatinRange 0.0 365.0)) false false)
  (Variables|Default|SetVelocity (* (Math|Vector|GetForwardVector _comet) (Variables|Default|GetSpeed))))

(fn ConstructionScript
  (bind _comet (Variables|Default|GetComet))
  (Components|StaticMesh|SetStaticMesh _comet (.OutItem (Utilities|Array|Random (Variables|Default|GetCometMesh))))
  (Rendering|Material|SetMaterial _comet 0 "/Game/Models/Asteroid/asteroids-pack-rocky-version/source/Material__3.Material__3")
  (Components|InstancedStaticMesh|AddInstance _comet (Math|Transform|MakeTransform "0, 0, 0" "0, 0, 0" "1.000000,1.000000,1.000000") false))