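; BP_SpaceGame keeps a running game timer and reports the player's score for the space game.
; On BeginPlay it caches the BP_SpaceGameInstance that holds PlayerScore.
; While TimerStart is true, Tick adds delta time to Timer and prints both the time and score as debug strings.
; The BeginGame event sets TimerStart to false, and nothing in these graphs sets it true.
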(event Custom|Begin%20Game
  (Variables|Default|SetbTimerStart false))

(event EventBeginPlay
  (bind _asbp_space_game_instance (Utilities|Casting|CastToBP_SpaceGameInstance (Game|GetGameInstance)))
  (Variables|Default|SetSpace%20Game%20Instance _asbp_space_game_instance))

(event EventTick
  (params (DeltaSeconds :type Float%20%28single-precision%29))
  (if (Variables|Default|GetbTimerStart)
    (bind _output_get (Variables|Default|SetTimer (+ DeltaSeconds (Variables|Default|GetTimer))))
    (Development|PrintString (Utilities|String|ToString(Float) _output_get) true true "(R=0.000000,G=0.660000,B=1.000000,A=1.000000)" 2.0 "Timer")
    (Development|PrintString (Utilities|String|ToString(Integer) (Variables|/Game/BluePrints/BP_SpaceGameInstance.BP_SpaceGameInstance_C|GetPlayerScore (Variables|Default|GetSpace%20Game%20Instance))) true true "(R=0.000000,G=0.660000,B=1.000000,A=1.000000)" 2.0 "PlayerSCore")))

(fn ConstructionScript)