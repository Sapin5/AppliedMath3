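; BP_Projectile is a simple projectile actor that moves in a straight line and destroys itself after a maximum lifetime.
; SetBulletVelocity stores the firing direction as the velocity.
; Each Tick adds that velocity as a world offset without sweep or delta-time scaling, so speed depends on frame rate and no collision is checked along the path.
; Tick also accumulates lifetime and destroys the actor once it exceeds MaxBulletLife.
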(event Custom|SetBulletVelocity
  (params (FiringDirection :type Vector))
  (Variables|Default|SetVelocity FiringDirection))

(event EventTick
  (params (DeltaSeconds :type Float%20%28single-precision%29))
  (Variables|Default|SetLifeTime (+ DeltaSeconds (Variables|Default|GetLifeTime)))
  (Transformation|AddActorWorldOffset (Variables|Default|GetVelocity))
  (if (> (Variables|Default|GetLifeTime) (Variables|Default|GetMaxBulletLife))
    (Actor|DestroyActor)))

(fn ConstructionScript)