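; Time checkpoint pickup for a space flying game that adds time to the game mode's timer, up to a cap, when the player plane overlaps it.
; On BeginPlay it caches game mode, game instance and player references and increments the checkpoint count.
; On overlap it spawns an actor at a random point in a large cube, then destroys itself.
; The construction script builds its visual as an instanced sphere mesh.
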(event OnComponentBeginOverlap(Sphere)
  (params (OverlappedComponent :type Primitive%20Component%20Object%20Reference) (OtherActor :type Actor%20Object%20Reference) (OtherComp :type Primitive%20Component%20Object%20Reference) (OtherBodyIndex :type Integer) (bFromSweep :type Boolean) (SweepResult :type Hit%20Result%20Structure%20%28by%20ref%29))
  (bind _space_game (Variables|Default|GetSpace%20Game))
  (Utilities|Casting|CastToBP_PlayerPlane OtherActor)
  (Variables|/Game/BluePrints/BP_SpaceGame.BP_SpaceGame_C|SetTimerDisplay _space_game (Math|Float|Clamp(Float) (+ (Variables|/Game/BluePrints/BP_SpaceGame.BP_SpaceGame_C|GetTimerDisplay _space_game) 1e+01) 0.0 6e+01))
  (Game|SpawnActorfromClass "BP_CheckPoint_Time_C" (Math|Transform|MakeTransform (Math|Vector|MakeVector (Math|Random|RandomFloatinRange -3.3e+04 3.3e+04) (Math|Random|RandomFloatinRange -3.3e+04 3.3e+04) (Math|Random|RandomFloatinRange -3.3e+04 3.3e+04))) "Undefined" "MultiplyWithRoot" 0 100 0)
  (Variables|Default|SetbCollided true)
  (Actor|DestroyActor))

(event EventBeginPlay
  (bind _asbp_space_game (Utilities|Casting|CastToBP_SpaceGame (Game|GetGameMode)))
  (Variables|Default|SetSpace%20Game _asbp_space_game)
  (bind _asbp_space_game_instance (Utilities|Casting|CastToBP_SpaceGameInstance (Game|GetGameInstance)))
  (Variables|Default|SetSpace%20Game%20Instance _asbp_space_game_instance)
  (bind _asbp_player_plane (Utilities|Casting|CastToBP_PlayerPlane (Game|Player|GetPlayerPawn 0)))
  (Variables|Default|SetAs%20BP%20Player%20Plane _asbp_player_plane)
  (Variables|/Game/BluePrints/BP_SpaceGame.BP_SpaceGame_C|SetCheckPointCount (Variables|Default|GetSpace%20Game) (+ (Variables|/Game/BluePrints/BP_SpaceGame.BP_SpaceGame_C|GetCheckPointCount (Variables|Default|GetSpace%20Game)) 1)))

(fn ConstructionScript
  (bind _pointsys (Variables|Default|GetPointSys))
  (Components|StaticMesh|SetStaticMesh _pointsys "/Game/BluePrints/Sphere.Sphere")
  (Rendering|Material|SetMaterial _pointsys 0 "/Game/Materials/M_Checkpoint_Time.M_Checkpoint_Time")
  (Components|InstancedStaticMesh|AddInstance _pointsys (Math|Transform|MakeTransform "0, 0, 0" "0, 0, 0" "1.000000,1.000000,1.000000") false))